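; BP_CAttachment_Warp is an attachment Blueprint in the action system that controls the visibility of a Warp component.
; It hides Warp on BeginPlay, shows it on equip and hides it again on unequip, calling the parent implementation first in each event.
; The visibility changes do not propagate to child components, and the construction script is empty.
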(event `self.ReceiveBeginPlay`
  (`parent.ReceiveBeginPlay`)
  (`SceneComponent.SetVisibility` (`self.Warp`) false false))

(event `self.OnEquip`
  (`parent.OnEquip`)
  (`SceneComponent.SetVisibility` (`self.Warp`) true false))

(event `self.OnUnEquip`
  (`parent.OnUnEquip`)
  (`SceneComponent.SetVisibility` (`self.Warp`) false false))

(fn `UserConstructionScript`)